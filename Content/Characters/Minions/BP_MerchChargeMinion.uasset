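; BP_MerchChargeMinion is a minion character that deals contact damage to BP_DarkPlayer and destroys itself on impact.
; On capsule overlap, it self-destructs against "Wall"-tagged actors, or damages whichever player component is active, checking Custgrand before Malbrev, then self-destructs.
; Self-destruct adds a backward and upward impulse, then destroys the actor after a short delay.
; Other overlapping actors only trigger a debug print.
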(event `self.CapsuleComponent.OnComponentBeginOverlap`
  (params (OverlappedComponent :type "PrimitiveComponent Object Reference") (OtherActor :type "Actor Object Reference") (OtherComp :type "PrimitiveComponent Object Reference") (OtherBodyIndex :type Integer) (bFromSweep :type Boolean) (SweepResult :type "HitResult Structure (by ref)"))
  (if (`self.ActorHasTag` OtherActor "Wall")
    (`self.SelfDestruct` :!label _label)
    (else
      (bind _asbp_dark_player (cast `/Game/Characters/Player/BP_DarkPlayer` OtherActor)
        (:`then`
          (bind _bpc_custgrand (`/Game/Characters/Player/BP_DarkPlayer.BPC_Custgrand` _asbp_dark_player))
          (if (`ActorComponent.IsActive` _bpc_custgrand)
            (`/Game/Characters/Player/BPC_Custgrand.TakeDamage` _bpc_custgrand 10.0)
            (goto _label)
            (else
              (bind _bpc_malbrev (`/Game/Characters/Player/BP_DarkPlayer.BPC_Malbrev` _asbp_dark_player))
              (if (`ActorComponent.IsActive` _bpc_malbrev)
                (`/Game/Characters/Player/BPC_Malbrev.Take Damage` _bpc_malbrev 10.0)
                (goto _label)))))
        (:`CastFailed`
          (`KismetSystemLibrary.PrintString` "Dat's not you!"))))))

(event `SelfDestruct`
  (bind (_returnvalue_x _returnvalue_y) (`KismetMathLibrary.BreakVector` (`self.GetActorForwardVector`)))
  (`CharacterMovementComponent.AddImpulse` (`self.CharacterMovement`) (`KismetMathLibrary.MakeVector` (* _returnvalue_x -10.0) (* _returnvalue_y -10.0) 200.0) false)
  (`KismetSystemLibrary.Delay` 0.5)
  (`self.K2_DestroyActor`))

(fn `UserConstructionScript`
  (`parent.UserConstructionScript`))