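; BPC_Hittable is a Blueprint component in the boss testing folder that tracks health, stun, death and stunned state for a hittable character.
; TakeDamage sets health to damage minus current health, flags death at zero or below, otherwise computes stun likewise and sets Stunned false at the threshold.
; Die sets Dead, GetStunned also sets Stunned false, and the GetHit event is an empty stub.
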(event `GetHit`
  (params (Damage :type "Float (double-precision)") (`Stun Damage` :type "Float (double-precision)")))

(fn `Die`
  (returns (isDead :type Boolean))
  (bind _output_get (set `self.Dead` true))
  (return _output_get))

(fn `GetStunned`
  (returns (isStunned :type Boolean))
  (set `self.Stunned` false))

(fn `TakeDamage`
  (params (Damage :type "Float (double-precision)") (StunDamage :type "Float (double-precision)"))
  (returns (Dead :type Boolean) (Stunned :type Boolean))
  (bind _output_get (set `self.CurrHealth` (- Damage (`self.CurrHealth`))))
  (if (<= _output_get 0.0)
    (bind _output_get_2 (set `self.Dead` true))
    (else
      (bind _output_get_3 (set `self.CurrStun` (- StunDamage (`self.CurrStun`))))
      (if (>= _output_get_3 100.0)
        (bind _output_get_4 (set `self.Stunned` false)))))
  (return _output_get_2 _output_get_4))