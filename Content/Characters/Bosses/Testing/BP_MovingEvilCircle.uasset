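; Boss testing hazard actor that moves a sphere and damages BP_DarkPlayer on overlap.
; On BeginPlay, a Timeline lerps Sphere's relative X position between two fixed offsets.
; Overlapping Sphere1 applies fixed damage to the player's active character component, checking BPCCustgrand first, then BPCMalbrev.
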(event `self.Sphere1.OnComponentBeginOverlap`
  (params (OverlappedComponent :type "PrimitiveComponent Object Reference") (OtherActor :type "Actor Object Reference") (OtherComp :type "PrimitiveComponent Object Reference") (OtherBodyIndex :type Integer) (bFromSweep :type Boolean) (SweepResult :type "HitResult Structure (by ref)"))
  (bind _asbp_dark_player (cast `/Game/Characters/Player/BP_DarkPlayer` OtherActor))
  (bind _bpc_custgrand (`/Game/Characters/Player/BP_DarkPlayer.BPC_Custgrand` _asbp_dark_player))
  (if (`ActorComponent.IsActive` _bpc_custgrand)
    (`/Game/Characters/Player/BPC_Custgrand.TakeDamage` _bpc_custgrand 10.0)
    (else
      (bind _bpc_malbrev (`/Game/Characters/Player/BP_DarkPlayer.BPC_Malbrev` _asbp_dark_player))
      (if (`ActorComponent.IsActive` _bpc_malbrev)
        (`/Game/Characters/Player/BPC_Malbrev.Take Damage` _bpc_malbrev 10.0)))))

(event `self.ReceiveBeginPlay`
  (bind (_direction _newtrack_0) (`Timeline|Timeline` :!via `PlayFromStart`)
    (:`Update`
      (`SceneComponent.K2_SetRelativeLocation` (`self.Sphere`) (`KismetMathLibrary.MakeVector` (`KismetMathLibrary.Lerp` 100.0 500.0 _newtrack_0)) false false))))

(fn `UserConstructionScript`)