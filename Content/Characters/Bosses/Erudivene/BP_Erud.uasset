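; Boss character Blueprint for Erudivene, extending a parent class's behavior.
; BeginPlay sets the attack animation to the basic swing montage, and Tick stores the distance to the player in DistanceToPlayer.
; SpawnChargeLimiter prints a debug message and spawns a BP_ChargeLimit at the boss's transform, adjusting for collisions but always spawning.
; LightningStrike is an empty stub.
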(event `self.ReceiveBeginPlay`
  (`parent.ReceiveBeginPlay`)
  (set `self.AttackAnimation` "/Game/Characters/Bosses/Erudivene/AM_Erud_BasicSwing.AM_Erud_BasicSwing"))

(event `self.ReceiveTick`
  (params (DeltaSeconds :type "Float (single-precision)"))
  (`parent.ReceiveTick` DeltaSeconds)
  (set `self.DistanceToPlayer` (`self.GetDistanceTo` (`GameplayStatics.GetPlayerCharacter` 0))))

(fn `LightningStrike`)

(fn `SpawnChargeLimiter`
  (`KismetSystemLibrary.PrintString` "I ran!")
  (`|SpawnActorFromClass` "/Game/Characters/Bosses/Erudivene/ErudHelperBPs/BP_ChargeLimit.BP_ChargeLimit_C" (`self.GetTransform`) "AdjustIfPossibleButAlwaysSpawn" "MultiplyWithRoot" null null))

(fn `UserConstructionScript`
  (`parent.UserConstructionScript`))