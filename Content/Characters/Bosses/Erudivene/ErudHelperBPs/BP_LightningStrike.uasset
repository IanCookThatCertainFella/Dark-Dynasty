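; BP_LightningStrike is an Erudivene boss helper actor that delivers a delayed lightning strike.
; Attack disables the damage cylinder's collision, waits two seconds, then HandSpawn swaps the visible cylinder and enables query collision until the actor destroys itself after the given Duration.
; Overlap with BP_DarkPlayer applies fixed damage to whichever of the Custgrand or Malbrev components is active, checking Custgrand first.
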(event `Attack`
  (params (Duration :type "Float (double-precision)" :default 5.0))
  (`PrimitiveComponent.SetCollisionEnabled` (`self.Cylinder1`) "NoCollision")
  (`KismetSystemLibrary.Delay` 2.0)
  (`self.HandSpawn`)
  (`KismetSystemLibrary.Delay` Duration)
  (`self.K2_DestroyActor`))

(event `self.ReceiveBeginPlay`)

(event `self.Cylinder1.OnComponentBeginOverlap`
  (params (OverlappedComponent :type "PrimitiveComponent Object Reference") (OtherActor :type "Actor Object Reference") (OtherComp :type "PrimitiveComponent Object Reference") (OtherBodyIndex :type Integer) (bFromSweep :type Boolean) (SweepResult :type "HitResult Structure (by ref)"))
  (bind _asbp_dark_player (cast `/Game/Characters/Player/BP_DarkPlayer` OtherActor)
    (:`then`
      (bind _bpc_custgrand (`/Game/Characters/Player/BP_DarkPlayer.BPC_Custgrand` _asbp_dark_player))
      (if (`ActorComponent.IsActive` _bpc_custgrand)
        (`/Game/Characters/Player/BPC_Custgrand.TakeDamage` _bpc_custgrand 10.0)
        (else
          (bind _bpc_malbrev (`/Game/Characters/Player/BP_DarkPlayer.BPC_Malbrev` _asbp_dark_player))
          (if (`ActorComponent.IsActive` _bpc_malbrev)
            (`/Game/Characters/Player/BPC_Malbrev.Take Damage` _bpc_malbrev 10.0)))))
    (:`CastFailed`
      (`KismetSystemLibrary.PrintString` "Dat's not you!"))))

(fn `HandSpawn`
  (bind _cylinder1 (`self.Cylinder1`))
  (`SceneComponent.SetHiddenInGame` (`self.Cylinder`) true false)
  (`SceneComponent.SetHiddenInGame` _cylinder1 false false)
  (`PrimitiveComponent.SetCollisionEnabled` _cylinder1 "QueryOnly"))

(fn `UserConstructionScript`)