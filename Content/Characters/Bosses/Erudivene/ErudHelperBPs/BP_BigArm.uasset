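; BP_BigArm is an arm attack for the Erudivene boss that rises from below and slams.
; Its Attack event opens BP_Lid, then chains timelines to raise the actor, rear back, slam, spin sideways and right itself.
; It then closes the lid and lowers the BigArm component with a reversed timeline.
; Capsule overlaps deal fixed damage to whichever BP_DarkPlayer character component is active, Custgrand or Malbrev.
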(event `self.ReceiveBeginPlay`)

(event `self.Capsule.OnComponentBeginOverlap`
  (params (OverlappedComponent :type "PrimitiveComponent Object Reference") (OtherActor :type "Actor Object Reference") (OtherComp :type "PrimitiveComponent Object Reference") (OtherBodyIndex :type Integer) (bFromSweep :type Boolean) (SweepResult :type "HitResult Structure (by ref)"))
  (bind _asbp_dark_player (cast `/Game/Characters/Player/BP_DarkPlayer` OtherActor)
    (:`then`
      (bind _bpc_custgrand (`/Game/Characters/Player/BP_DarkPlayer.BPC_Custgrand` _asbp_dark_player))
      (if (`ActorComponent.IsActive` _bpc_custgrand)
        (`/Game/Characters/Player/BPC_Custgrand.TakeDamage` _bpc_custgrand 10.0)
        (else
          (bind _bpc_malbrev (`/Game/Characters/Player/BP_DarkPlayer.BPC_Malbrev` _asbp_dark_player))
          (if (`ActorComponent.IsActive` _bpc_malbrev)
            (`/Game/Characters/Player/BPC_Malbrev.Take Damage` _bpc_malbrev 10.0)))))
    (:`CastFailed`
      (`KismetSystemLibrary.PrintString` "Dat's not you!"))))

(event `Slam`)

(event `Attack`
  (`KismetSystemLibrary.PrintString` "Arm Attack!")
  (`KismetSystemLibrary.Delay` 1.0)
  (bind _returnvalue (`GameplayStatics.GetActorOfClass` "/Game/Levels/Erudivene/BP_Lid.BP_Lid_C"))
  (bind _output_get (set `self.Lid` _returnvalue))
  (`/Game/Levels/Erudivene/BP_Lid.Open` _output_get)
  (bind (_direction _newtrack_0) (`Timeline|RaiseUpTimeline` :!via `PlayFromStart`)
    (:`Update`
      (`self.K2_SetActorLocation` (`KismetMathLibrary.MakeVector` 0.0 0.0 (`KismetMathLibrary.Lerp` -1000.0 0.0 _newtrack_0))))
    (:`Finished`
      (`KismetSystemLibrary.Delay` 0.2)
      (bind (_direction_2 _newtrack_0_2) (`Timeline|RearBackTimeline` :!via `PlayFromStart`)
        (:`Update`
          (`self.K2_SetActorRotation` (`KismetMathLibrary.MakeRotator` (`KismetMathLibrary.Lerp` 0.0 -20.0 _newtrack_0_2))))
        (:`Finished`
          (bind (_direction_3 _newtrack_0_3) (`Timeline|SlamTimeline` :!via `PlayFromStart`)
            (:`Update`
              (`self.K2_SetActorRotation` (`KismetMathLibrary.MakeRotator` (`KismetMathLibrary.Lerp` -20.0 90.0 _newtrack_0_3))))
            (:`Finished`
              (`KismetSystemLibrary.Delay` 0.4)
              (bind (_direction_4 _newtrack_0_4) (`Timeline|SpinTimeline` :!via `PlayFromStart`)
                (:`Update`
                  (`self.K2_SetActorRotation` (`KismetMathLibrary.MakeRotator` 90.0 0.0 (`KismetMathLibrary.Lerp` 0.0 90.0 _newtrack_0_4))))
                (:`Finished`
                  (bind (_direction_5 _newtrack_0_5) (`Timeline|RaiseTimeline` :!via `PlayFromStart`)
                    (:`Update`
                      (`self.K2_SetActorRotation` (`KismetMathLibrary.MakeRotator` (`KismetMathLibrary.Lerp` 90.0 0.0 _newtrack_0_5))))
                    (:`Finished`
                      (`/Game/Levels/Erudivene/BP_Lid.Close` (`self.Lid`))
                      (bind (_direction_6 _newtrack_0_6) (`Timeline|Timeline` :!via `ReverseFromEnd`)
                        (:`Update`
                          (`SceneComponent.K2_SetRelativeLocation` (`self.BigArm`) (`KismetMathLibrary.MakeVector` 0.0 0.0 (`KismetMathLibrary.Lerp` -1000.0 0.0 _newtrack_0_6)) false false))))))))))))))

(fn `UserConstructionScript`)