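; BP_ElementalBall is a helper for the Erudivene boss: a homing projectile that chases and damages the player.
; Its Chase event uses AI MoveTo toward the player character, and is not called within this Blueprint.
; Overlapping BP_DarkPlayer deals damage through whichever of the Custgrand or Malbrev components is active, then destroys the ball.
; Otherwise it expires once a per-tick, frame-rate-dependent counter reaches PopTimer.
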(event `self.ReceiveTick`
  (params (DeltaSeconds :type "Float (single-precision)"))
  (if (>= (`self.Timer`) (`self.PopTimer`))
    (`self.K2_DestroyActor`)
    (else
      (set `self.Timer` (+ (`self.Timer`) 0.1)))))

(event `Chase`
  (`KismetSystemLibrary.PrintString` "Go Get'em!")
  (`AITask_MoveTo.AIMoveTo` (`AIBlueprintHelperLibrary.GetAIController` self) (0.0 0.0 0.0) (`GameplayStatics.GetPlayerCharacter` 0)
    (:`OnRequestFailed`
      (`KismetSystemLibrary.PrintString` "Can't do it!"))))

(event `self.ReceiveActorBeginOverlap`
  (params (OtherActor :type "Actor Object Reference"))
  (bind _asbp_dark_player (cast `/Game/Characters/Player/BP_DarkPlayer` OtherActor)
    (:`then`
      (bind _bpc_custgrand (`/Game/Characters/Player/BP_DarkPlayer.BPC_Custgrand` _asbp_dark_player))
      (if (`ActorComponent.IsActive` _bpc_custgrand)
        (`/Game/Characters/Player/BPC_Custgrand.TakeDamage` _bpc_custgrand 10.0)
        (`self.K2_DestroyActor` :!label _label)
        (else
          (bind _bpc_malbrev (`/Game/Characters/Player/BP_DarkPlayer.BPC_Malbrev` _asbp_dark_player))
          (if (`ActorComponent.IsActive` _bpc_malbrev)
            (`/Game/Characters/Player/BPC_Malbrev.Take Damage` _bpc_malbrev 10.0)
            (goto _label)))))
    (:`CastFailed`
      (`KismetSystemLibrary.PrintString` "Dat's not you!"))))

(fn `UserConstructionScript`)