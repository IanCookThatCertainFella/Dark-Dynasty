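; Base boss enemy Blueprint that smoothly rotates to face the player unless Locked, and tracks health, stun buildup, death and a second phase.
; GetDamaged reduces health, fills stun until Stunned, plays a hit reaction while stunned, and sets SecondPhase at half health.
; The stun-hit montage leads into a stun montage that loops while Stunned.
; Die starts the death montage and destroys the actor immediately, without waiting.
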(event `self.ReceiveBeginPlay`)

(event `self.ReceiveTick`
  (params (DeltaSeconds :type "Float (single-precision)"))
  (if (!= (`self.Locked`) true)
    (`self.K2_SetActorRotation` (`KismetMathLibrary.RInterpTo` (`self.K2_GetActorRotation`) (`KismetMathLibrary.FindLookAtRotation` (`self.K2_GetActorLocation`) (`self.K2_GetActorLocation` (`GameplayStatics.GetPlayerPawn` 0))) DeltaSeconds 5.0))))

(event `self.ReceiveAnyDamage`
  (params (Damage :type "Float (single-precision)") (DamageType :type "DamageType Object Reference") (InstigatedBy :type "Controller Object Reference") (DamageCauser :type "Actor Object Reference")))

(event `PlayStunHitMontage`
  (set `self.GettingStunHit` true)
  (`|PlayMontage` (`self.Mesh`) (`self.StunHit`)
    (:`OnCompleted`
      (set `self.GettingStunHit` false)
      (`self.PlayStunMontage`))))

(event `PlayStunMontage`
  (`|PlayMontage` (`self.Mesh`) (`self.Stun`) :!label _label
    (:`OnCompleted`
      (if (`self.Stunned`)
        (goto _label)))))

(fn `Die`
  (`self.PlayAnimMontage` (`self.Death`))
  (`self.K2_DestroyActor`))

(fn `GetDamaged`
  (params (Damage :type "Float (double-precision)") (StunDamage :type "Float (double-precision)"))
  (`KismetSystemLibrary.PrintString` "ow")
  (bind _output_get (set `self.CurrHealth` (- (`self.CurrHealth`) Damage)))
  (if (<= _output_get 0.0)
    (set `self.Dead` true)
    (`self.Die`)
    (else
      (if (not (`self.Stunned`))
        (bind _output_get_2 (set `self.CurrStun` (+ StunDamage (`self.CurrStun`))))
        (if (>= _output_get_2 100.0)
          (set `self.Stunned` true))
        (else
          (`self.PlayStunHitMontage`)))
      (if (<= (`self.CurrHealth`) (/ (`self.MaxHealth`) 2.0))
        (set `self.SecondPhase` true)))))

(fn `UserConstructionScript`)