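; Boss helper actor for telegraphed, delayed area attacks that damage BP_DarkPlayer, either by falling projectile or by hands.
; SpawnProjectile reveals DamageArea after a random delay and separately spawns an owned projectile overhead, whose overlap triggers a sphere-trace explosion.
; HandsAttack shows DamageArea, swaps it for colliding Hands after a delay, then destroys itself.
; Damage routes to whichever Custgrand or Malbrev component is active; the particle function is empty.
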(event `SpawnProjectile`
  (params (TravelTime :type "Float (double-precision)" :default 3.0) (Random :type Boolean))
  (bind _returnvalue (`self.GetTransform`))
  (`self.Reveal`)
  (if Random
    (`KismetSystemLibrary.Delay` (+ TravelTime (`KismetMathLibrary.RandomFloatInRange` 0.0 0.5)))
    (else
      (`KismetSystemLibrary.Delay` TravelTime)))
  (`|SpawnActorFromClass` "/Game/Characters/Bosses/BaseEnemy/BaseEnemyHelpers/BP_BaseFallingProjectile.BP_BaseFallingProjectile_C" (`KismetMathLibrary.MakeTransform` (`KismetMathLibrary.MakeVector` (.x (.location _returnvalue)) (.y (.location _returnvalue)) (+ (.z (.location _returnvalue)) 500.0)) (.rotation _returnvalue) (.scale _returnvalue)) "Undefined" "MultiplyWithRoot" self null))

(event `Reveal`
  (`KismetSystemLibrary.Delay` (`KismetMathLibrary.RandomFloatInRange` 0.2 2.0))
  (`SceneComponent.SetHiddenInGame` (`self.DamageArea`) false false))

(event `self.ReceiveBeginPlay`)

(event `HandsAttack`
  (params (Delay :type "Float (double-precision)" :default 2.0) (Duration :type "Float (double-precision)" :default 5.0))
  (`SceneComponent.SetHiddenInGame` (`self.DamageArea`) false false)
  (`KismetSystemLibrary.Delay` Delay)
  (`self.SpawnHands`)
  (`KismetSystemLibrary.Delay` Duration)
  (`self.RemoveHands`))

(event `self.Hands.OnComponentBeginOverlap`
  (params (OverlappedComponent :type "PrimitiveComponent Object Reference") (OtherActor :type "Actor Object Reference") (OtherComp :type "PrimitiveComponent Object Reference") (OtherBodyIndex :type Integer) (bFromSweep :type Boolean) (SweepResult :type "HitResult Structure (by ref)"))
  (bind _asbp_dark_player (cast `/Game/Characters/Player/BP_DarkPlayer` OtherActor)
    (:`then`
      (bind _bpc_custgrand (`/Game/Characters/Player/BP_DarkPlayer.BPC_Custgrand` _asbp_dark_player))
      (if (`ActorComponent.IsActive` _bpc_custgrand)
        (`/Game/Characters/Player/BPC_Custgrand.TakeDamage` _bpc_custgrand 10.0)
        (else
          (bind _bpc_malbrev (`/Game/Characters/Player/BP_DarkPlayer.BPC_Malbrev` _asbp_dark_player))
          (if (`ActorComponent.IsActive` _bpc_malbrev)
            (`/Game/Characters/Player/BPC_Malbrev.Take Damage` _bpc_malbrev 10.0)))))
    (:`CastFailed`
      (`KismetSystemLibrary.PrintString` "Dat's not you!"))))

(event `self.DamageArea.OnComponentBeginOverlap`
  (params (OverlappedComponent :type "PrimitiveComponent Object Reference") (OtherActor :type "Actor Object Reference") (OtherComp :type "PrimitiveComponent Object Reference") (OtherBodyIndex :type Integer) (bFromSweep :type Boolean) (SweepResult :type "HitResult Structure (by ref)"))
  (bind _asbp_base_falling_projectile (cast `/Game/Characters/Bosses/BaseEnemy/BaseEnemyHelpers/BP_BaseFallingProjectile` OtherActor))
  (if (== (`self.GetOwner` _asbp_base_falling_projectile) self)
    (`self.K2_DestroyActor`)
    (`self.SpawnExplosionParticle`)
    (`self.SpawnExplosion` (`self.ExplosionSize`))
    (`self.K2_DestroyActor`)
    (else
      (`KismetSystemLibrary.PrintString` "You are not the father"))))

(fn `RemoveHands`
  (`self.K2_DestroyActor`))

(fn `SpawnExplosion`
  (params (Size :type "Float (double-precision)" :default 200.0))
  (bind _returnvalue (`self.K2_GetActorLocation`))
  (`KismetSystemLibrary.PrintString` "Hello")
  (bind (_outhit _returnvalue_2) (`KismetSystemLibrary.SphereTraceSingleForObjects` :`Start` _returnvalue :`End` _returnvalue :`Radius` Size :`ObjectTypes` (`|MakeArray` "ObjectTypeQuery3" :!type "EObjectTypeQuery Enum") :`DrawDebugType` "Persistent"))
  (if _returnvalue_2
    (bind _asbp_dark_player (cast `/Game/Characters/Player/BP_DarkPlayer` (`.HitActor` (`GameplayStatics.BreakHitResult` _outhit)))
      (:`then`
        (bind _bpc_custgrand (`/Game/Characters/Player/BP_DarkPlayer.BPC_Custgrand` _asbp_dark_player))
        (if (`ActorComponent.IsActive` _bpc_custgrand)
          (`/Game/Characters/Player/BPC_Custgrand.TakeDamage` _bpc_custgrand 10.0)
          (else
            (bind _bpc_malbrev (`/Game/Characters/Player/BP_DarkPlayer.BPC_Malbrev` _asbp_dark_player))
            (if (`ActorComponent.IsActive` _bpc_malbrev)
              (`/Game/Characters/Player/BPC_Malbrev.Take Damage` _bpc_malbrev 10.0)))))
      (:`CastFailed`
        (`KismetSystemLibrary.PrintString` "Dat's not you!")))))

(fn `SpawnExplosionParticle`)

(fn `SpawnHands`
  (bind _damagearea (`self.DamageArea`))
  (bind _hands (`self.Hands`))
  (`SceneComponent.SetHiddenInGame` _damagearea true false)
  (`PrimitiveComponent.SetCollisionEnabled` _damagearea "NoCollision")
  (`SceneComponent.SetHiddenInGame` _hands false false)
  (`PrimitiveComponent.SetCollisionEnabled` _hands "QueryOnly")
  (`KismetSystemLibrary.PrintString` "Hands!"))

(fn `UserConstructionScript`
  (`PrimitiveComponent.SetCollisionEnabled` (`self.Hands`) "NoCollision"))