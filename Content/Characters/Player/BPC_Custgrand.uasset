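; Player combat component for the Custgrand character, handling light, chargeable heavy and special attacks, parry, damage reactions and swapping while setting Actionable locks on itself and its owner.
; Light and heavy attacks damage enemies through a sphere-trace hitbox, with heavy charge widening the radius.
; Special charge drains the owner's bar and powers a dash punch, sharing CurrCharge with heavy in a separate value band.
; Successful parries grant brief invincibility; unarmored hits cause knockback.
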(event `self.ReceiveTick`
  (params (DeltaSeconds :type "Float (single-precision)")))

(event `EnhancedInput|/Game/Inputs/IA_LightAttack`
  (params (ActionValue :type Boolean) (ElapsedSeconds :type "Float (double-precision)") (TriggeredSeconds :type "Float (double-precision)") (InputAction :type "InputAction Object Reference" :default "/Game/Inputs/IA_LightAttack.IA_LightAttack"))
  ; Light Attack
  (:`Completed`
    (if (`self.IsActive`)
      (if (`self.Actionable`)
        (set `/Game/Characters/Player/BP_DarkPlayer.Actionable` false (`self.Owner`))
        (set `self.Actionable` false)
        (`KismetSystemLibrary.PrintString` "Big Swing!")
        (`self.Spawn Hitbox` (`self.LightAttackSize`) (`self.LightAttackDamage`))
        (`KismetSystemLibrary.Delay` (`self.LightAttackCooldown`))
        (set `self.Actionable` true)
        (set `/Game/Characters/Player/BP_DarkPlayer.Actionable` true (`self.Owner`))))))

(event `EnhancedInput|/Game/Inputs/IA_ChargeableHeavy`
  (params (ActionValue :type Boolean) (ElapsedSeconds :type "Float (double-precision)") (TriggeredSeconds :type "Float (double-precision)") (InputAction :type "InputAction Object Reference" :default "/Game/Inputs/IA_ChargeableHeavy.IA_ChargeableHeavy"))
  (bind _currcharge (`self.CurrCharge`))
  ; Heavy Attack
  (:`Ongoing`
    (if (`self.IsActive`)
      (if (and (> _currcharge 0.0) (< _currcharge 10.0))
        (bind _output_get (set `self.CurrCharge` (+ (`self.CurrCharge`) (`self.ChargeRate`)) :!label _label))
        (if (`KismetMathLibrary.InRange_FloatFloat` _output_get (+ (`self.HeavyAttackCharge1`) -0.01) (`self.HeavyAttackCharge1`))
          (`KismetSystemLibrary.PrintString` "Charge1")
          (set `self.HeavyAttackSize` 450.0))
        (if (`KismetMathLibrary.InRange_FloatFloat` (`self.CurrCharge`) (+ (`self.HeavyAttackCharge2`) -0.01) (`self.HeavyAttackCharge2`))
          (set `self.HeavyAttackSize` 750.0)
          (`KismetSystemLibrary.PrintString` "Charge2"))
        (set `self.Actionable` false)
        (set `/Game/Characters/Player/BP_DarkPlayer.Actionable` false (`self.Owner`))
        (elif (`self.Actionable`)
          (goto _label)))))
  (:`Canceled`
    (if (`self.IsActive`)
      (if (> (`self.CurrCharge`) 0.0)
        (`self.Spawn Hitbox` (`self.HeavyAttackSize`) (`self.HeavyAttackDamage`))
        (set `self.CurrCharge` 0.0)
        (set `self.HeavyAttackSize` 150.0)
        (`KismetSystemLibrary.Delay` (`self.HeavyAttackCooldown`))
        (set `self.Actionable` true)
        (set `/Game/Characters/Player/BP_DarkPlayer.Actionable` true (`self.Owner`)))))
  (:`Completed`
    (if (`self.IsActive`)
      (if (> (`self.CurrCharge`) 0.0)
        (set `self.CurrCharge` 0.0)
        (`KismetSystemLibrary.Delay` (`self.HeavyAttackCooldown`))
        (set `self.Actionable` true)
        (set `/Game/Characters/Player/BP_DarkPlayer.Actionable` true (`self.Owner`))))))

(event `EnhancedInput|/Game/Inputs/IA_ChargeableSpecial`
  (params (ActionValue :type Boolean) (ElapsedSeconds :type "Float (double-precision)") (TriggeredSeconds :type "Float (double-precision)") (InputAction :type "InputAction Object Reference" :default "/Game/Inputs/IA_ChargeableSpecial.IA_ChargeableSpecial"))
  (bind _currcharge (`self.CurrCharge`))
  (bind _currcharge_2 (`self.CurrCharge`))
  ; Special Attack
  (:`Ongoing`
    (if (`self.IsActive`)
      (if (and (> _currcharge_2 10.0) (< _currcharge_2 100.0))
        (if (>= (`/Game/Characters/Player/BP_DarkPlayer.CustSpecialBar` (`self.Owner`)) (`self.SpecialCost`)) :!label _label_2
          (if (< (`self.CurrCharge`) 10.0)
            (set `self.CurrCharge` 10.0))
          (set `/Game/Characters/Player/BP_DarkPlayer.CustSpecialBar` (- (`/Game/Characters/Player/BP_DarkPlayer.CustSpecialBar` (`self.Owner`)) (`self.SpecialCost`)) (`self.Owner`))
          (bind _output_get (set `self.CurrCharge` (+ (`self.CurrCharge`) (`self.ChargeRate`))))
          (if (`KismetMathLibrary.InRange_FloatFloat` _output_get (+ (`self.SpecialAttackCharge1`) -0.01) (`self.SpecialAttackCharge1`))
            (`KismetSystemLibrary.PrintString` "Charge1"))
          (if (`KismetMathLibrary.InRange_FloatFloat` (`self.CurrCharge`) (+ (`self.SpecialAttackCharge2`) -0.01) (`self.SpecialAttackCharge2`))
            (`KismetSystemLibrary.PrintString` "Charge2"))
          (set `self.Actionable` false)
          (elif (and (> _currcharge 10.0) (< _currcharge 100.0))
            (`/Engine/EditorBlueprintResources/StandardMacros.DoOnce` false :!label _label_3
              (:`Completed`
                (`KismetSystemLibrary.PrintString` "Forced big special swing")
                (set `self.CurrCharge` 0.0)
                (`KismetSystemLibrary.Delay` (`self.SpecialAttackCooldown`))
                (set `self.Actionable` true)))
            (else
              (`KismetSystemLibrary.PrintString` "No Big Special Swing"))))
        (elif (`self.Actionable`)
          (goto _label_2)))))
  (:`Canceled`
    (if (`self.IsActive`)
      (if (< (`/Game/Characters/Player/BP_DarkPlayer.CustSpecialBar` (`self.Owner`)) 0.9)
        (set `self.CurrCharge` 0.0)
        (`KismetSystemLibrary.Delay` (`self.SpecialAttackCooldown`))
        (set `self.Actionable` true)
        (set `/Game/Characters/Player/BP_DarkPlayer.Actionable` true (`self.Owner`))
        (goto _label_3 :!via `Reset`)
        (else
          (`self.Special Punch` (`self.CurrCharge`))
          (set `self.CurrCharge` 0.0)
          (`KismetSystemLibrary.Delay` (`self.SpecialAttackCooldown`))
          (set `self.Actionable` true)
          (set `/Game/Characters/Player/BP_DarkPlayer.Actionable` true (`self.Owner`))
          (goto _label_3 :!via `Reset`)))))
  (:`Completed`
    (if (`self.IsActive`)
      (if (> (`self.CurrCharge`) 0.0)
        (set `self.CurrCharge` 0.0)
        (`KismetSystemLibrary.Delay` (`self.SpecialAttackCooldown`))
        (set `self.Actionable` true)
        (set `/Game/Characters/Player/BP_DarkPlayer.Actionable` true (`self.Owner`))))))

(event `EnhancedInput|/Game/Input/Actions/IA_Parry`
  (params (ActionValue :type Boolean) (ElapsedSeconds :type "Float (double-precision)") (TriggeredSeconds :type "Float (double-precision)") (InputAction :type "InputAction Object Reference" :default "/Game/Input/Actions/IA_Parry.IA_Parry"))
  (:`Completed`
    (if (`self.IsActive`)
      (set `self.Parry` true)
      (set `self.Actionable` false)
      (`KismetSystemLibrary.PrintString` "Parry!")
      (`KismetSystemLibrary.Delay` 0.2)
      (set `self.Parry` false)
      (`KismetSystemLibrary.PrintString` "Parry Done!")
      (`KismetSystemLibrary.Delay` 0.5)
      (set `self.Actionable` true)
      (set `/Game/Characters/Player/BP_DarkPlayer.Actionable` true (`self.Owner`)))))

(event `EnhancedInput|/Game/Inputs/IA_Swap`
  (params (ActionValue :type Boolean) (ElapsedSeconds :type "Float (double-precision)") (TriggeredSeconds :type "Float (double-precision)") (InputAction :type "InputAction Object Reference" :default "/Game/Inputs/IA_Swap.IA_Swap"))
  (:`Completed`
    (if (`self.Actionable`)
      (`KismetSystemLibrary.PrintString` "Big Swap")
      (`/Game/Characters/Player/BP_DarkPlayer.Swap` (`self.Owner`)))))

(event `TakeDamage`
  (params (Damage :type "Float (double-precision)"))
  (bind _owner (`self.Owner`))
  (bind _returnvalue (- (`self.Health`) Damage))
  (`KismetSystemLibrary.PrintString` "Y'owhch!")
  (if (`self.IsActive`)
    (if (`self.Invincible`)
      (`KismetSystemLibrary.PrintString` "Tink")
      (elif (`self.Parry`)
        (set `self.Invincible` true)
        (`KismetSystemLibrary.Delay` 2.0)
        (set `self.Invincible` false)
        (`KismetSystemLibrary.PrintString` "Paryy!!!!!")
        (elif (`self.Armor`)
          (set `self.Health` _returnvalue)
          (else
            (bind _output_get (set `self.Health` _returnvalue))
            (if (<= _output_get 0.0)
              (`self.Die`)
              (else
                (`KismetSystemLibrary.PrintString` "Yowch!!!")
                (set `self.Actionable` false)
                (`CharacterMovementComponent.AddImpulse` (`Character.CharacterMovement` _owner) (* (+ (`Actor.GetActorForwardVector` _owner) (0.0 0.0 1.0)) (-1500.0 -1500.0 500.0)) true)
                (`KismetSystemLibrary.Delay` 0.5)
                (set `self.Actionable` true)))))))))

(event `Key|One`
  (params (Key :type "Key Structure"))
  (:`Pressed`
    (`self.Special Punch` 0.0)))

(event `Special Punch`
  (params (ChargeAmount :type "Float (double-precision)"))
  (bind _owner (`self.Owner`))
  (bind _owner_2 (`self.Owner`))
  (bind _charactermovement (`Character.CharacterMovement` _owner_2))
  (`KismetSystemLibrary.PrintString` "Hello")
  (if (>= ChargeAmount 11.0)
    (`KismetSystemLibrary.PrintString` "Yes?")
    (if (>= ChargeAmount 12.0)
      (set `self.SpecialDistance` (4500.0 4500.0 0.0))
      (`KismetSystemLibrary.PrintString` "Go Away")
      (set `self.SpecialAttackCooldown` 1.0)
      (else
        (set `self.SpecialDistance` (3000.0 3000.0 0.0))
        (`KismetSystemLibrary.PrintString` "Welcome!")
        (set `self.SpecialAttackCooldown` 0.5))))
  (set `CharacterMovementComponent.GravityScale` 0.0 _charactermovement)
  (set `self.Actionable` false)
  (set `/Game/Characters/Player/BP_DarkPlayer.Actionable` false (`self.Owner`))
  (`CharacterMovementComponent.AddImpulse` _charactermovement (* (`Actor.GetActorForwardVector` _owner_2) (`self.SpecialDistance`)) true)
  (`self.Activate` (`/Game/Characters/Player/BP_DarkPlayer.SpecialPunch` _owner) false)
  (set `CharacterMovementComponent.GravityScale` 2.5 (`Character.CharacterMovement` _owner))
  (set `self.SpecialDistance` (1500.0 1500.0 0.0))
  (`KismetSystemLibrary.Delay` (`self.SpecialAttackCooldown`))
  (set `self.SpecialAttackCooldown` 0.5)
  (set `/Game/Characters/Player/BP_DarkPlayer.Actionable` true (`self.Owner`))
  (set `self.Actionable` true))

(event `Die`)

(fn `Spawn Hitbox`
  (params (Radius :type "Float (double-precision)") (Damage :type "Float (double-precision)"))
  (bind _returnvalue (`SceneComponent.K2_GetComponentLocation` (`/Game/Characters/Player/BP_DarkPlayer.HitboxArea` (`self.Owner`))))
  (bind (_outhit _returnvalue_2) (`KismetSystemLibrary.SphereTraceSingleForObjects` :`Start` _returnvalue :`End` _returnvalue :`Radius` Radius :`ObjectTypes` (`|MakeArray` "ObjectTypeQuery3" :!type "EObjectTypeQuery Enum") :`DrawDebugType` "Persistent"))
  (if _returnvalue_2
    (bind (_bblockinghit _binitialoverlap _time _distance _location _impactpoint _normal _impactnormal _physmat _hitactor) (`GameplayStatics.BreakHitResult` _outhit))
    (if (`Actor.ActorHasTag` _hitactor "Enemy")
      (bind _asbp_base_enemy (cast `/Game/Characters/Bosses/BaseEnemy/BP_BaseEnemy` _hitactor)
        (:`then`
          (`/Game/Characters/Bosses/BaseEnemy/BP_BaseEnemy.GetDamaged` _asbp_base_enemy Damage 10.0))
        (:`CastFailed`
          (`KismetSystemLibrary.PrintString` "Owch")))
      (else
        (`KismetSystemLibrary.PrintString` "Tang")))
    (else
      (`KismetSystemLibrary.PrintString` "Whoosh"))))