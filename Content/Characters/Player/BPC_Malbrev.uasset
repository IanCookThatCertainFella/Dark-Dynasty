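; Player character component for Malbrev that handles light, heavy and special attack inputs plus a character swap.
; Each attack clears a shared Actionable flag and restores it after its own cooldown delay, while swap calls Swap on the owner.
; Attacks only print placeholder text, and SpawnHitbox and SpawnProjectile are empty stubs.
; The special spends CurrSpecial only when it is below SpecialCost, so the resource check appears inverted.
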(event `EnhancedInput|/Game/Inputs/IA_LightAttack`
  (params (ActionValue :type Boolean) (ElapsedSeconds :type "Float (double-precision)") (TriggeredSeconds :type "Float (double-precision)") (InputAction :type "InputAction Object Reference" :default "/Game/Inputs/IA_LightAttack.IA_LightAttack"))
  (:`Triggered`
    (if (`self.Actionable`)
      (set `self.Actionable` false)
      (`KismetSystemLibrary.PrintString` "Tiny Swing!")
      (`KismetSystemLibrary.Delay` (`self.LightAttackCooldown`))
      (set `self.Actionable` true))))

(event `EnhancedInput|/Game/Inputs/IA_HeavyAttack`
  (params (ActionValue :type Boolean) (ElapsedSeconds :type "Float (double-precision)") (TriggeredSeconds :type "Float (double-precision)") (InputAction :type "InputAction Object Reference" :default "/Game/Inputs/IA_HeavyAttack.IA_HeavyAttack"))
  (:`Triggered`
    (if (`self.Actionable`)
      (set `self.Actionable` false)
      (`KismetSystemLibrary.PrintString` "Less Tiny Swing!!")
      (`KismetSystemLibrary.Delay` (`self.HeavyAttackCooldown`))
      (set `self.Actionable` true))))

(event `EnhancedInput|/Game/Inputs/IA_SpecialAttack`
  (params (ActionValue :type Boolean) (ElapsedSeconds :type "Float (double-precision)") (TriggeredSeconds :type "Float (double-precision)") (InputAction :type "InputAction Object Reference" :default "/Game/Inputs/IA_SpecialAttack.IA_SpecialAttack"))
  (:`Triggered`
    (if (`self.Actionable`)
      (set `self.Actionable` false)
      (if (< (`self.CurrSpecial`) (`self.SpecialCost`))
        (set `self.CurrSpecial` (- (`self.CurrSpecial`) (`self.SpecialCost`)))
        (`KismetSystemLibrary.PrintString` "Special tiny swing")
        (`KismetSystemLibrary.Delay` (`self.SpecialAttackCooldown`))
        (set `self.Actionable` true)
        (else
          (`KismetSystemLibrary.PrintString` "No special tiny swing")
          (`KismetSystemLibrary.Delay` (`self.SpecialAttackCooldown`))
          (set `self.Actionable` true))))))

(event `EnhancedInput|/Game/Inputs/IA_Swap`
  (params (ActionValue :type Boolean) (ElapsedSeconds :type "Float (double-precision)") (TriggeredSeconds :type "Float (double-precision)") (InputAction :type "InputAction Object Reference" :default "/Game/Inputs/IA_Swap.IA_Swap"))
  (:`Completed`
    (if (`self.Actionable`)
      (`KismetSystemLibrary.PrintString` "Yo!")
      (`/Game/Characters/Player/BP_DarkPlayer.Swap` (`self.Owner`)))))

(fn `Spawn Hitbox`)

(fn `Spawn Projectile`)